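; BP_SecurityDoor is a security door that swings open on a timeline and reports to the BP_Gates manager.
; It finds the first BP_Gates actor at BeginPlay and stores it as its manager.
; UnlockDoor plays the timeline, while OpenDoor and Interact restart it from the beginning.
; The timeline lerps the DoorHinge rotation and calls SubDoorOpened on the manager every update and again on finish.
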(event Custom|UnlockDoor
  (bind _alpha (Timeline|DoorOpenTimeline Play)
    (:Update
      (Transformation|SetRelativeRotation (Variables|Default|GetDoorHinge) (Math|Rotator|Lerp(Rotator) "0, 0, 0" "300.000000,90.000000,300.000000" _alpha) false false))
    (:Finished
      _))
  (Default|SubDoorOpened (Variables|Default|GetManagerRef)))

(event Custom|OpenDoor
  (bind _alpha (Timeline|DoorOpenTimeline PlayFromStart)
    (:Update
      (Transformation|SetRelativeRotation (Variables|Default|GetDoorHinge) (Math|Rotator|Lerp(Rotator) "0, 0, 0" "300.000000,90.000000,300.000000" _alpha) false false))
    (:Finished
      _))
  (Default|SubDoorOpened (Variables|Default|GetManagerRef)))

(event Collision|EventActorBeginOverlap
  (params (OtherActor :type Actor%20Object%20Reference)))

(event EventTick
  (params (DeltaSeconds :type Float%20%28single-precision%29)))

(event EventBeginPlay
  (bind _returnvalue (Actor|GetActorOfClass "/Game/BP_Gates.BP_Gates_C"))
  (Variables|Default|SetManagerRef _returnvalue))

(event EventInteract
  (bind _alpha (Timeline|DoorOpenTimeline PlayFromStart)
    (:Update
      (Transformation|SetRelativeRotation (Variables|Default|GetDoorHinge) (Math|Rotator|Lerp(Rotator) "0, 0, 0" "300.000000,90.000000,300.000000" _alpha) false false))
    (:Finished
      _))
  (Default|SubDoorOpened (Variables|Default|GetManagerRef)))

(fn ConstructionScript)