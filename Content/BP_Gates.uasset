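; BP_Gates is a gate actor that keeps a security door locked until a first door has been triggered.
; SubDoorOpened or SecurityDoorA_Pressed sets a flag that lets SecurityDoorB_Pressed swing the mesh 90 degrees on a timeline, otherwise printing "Locked".
; DoorOfficeOpened is meant to message a main door from an opened-door count, but never increments it and its contradictory nested checks cannot both pass.
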(event Custom|SubDoorOpened
  (Variables|Default|SetIsDoorA_Opened true))

(event Custom|SecurityDoorA_Pressed
  (Variables|Default|SetIsDoorA_Opened true))

(event Custom|SecurityDoorB_Pressed
  (if (Variables|Default|GetIsDoorA_Opened)
    (bind _alpha (Timeline|DoorOpenTimeline PlayFromStart)
      (:Update
        (Transformation|SetRelativeRotation (Variables|Default|GetStaticMesh) (Math|Rotator|Lerp(Rotator) "0.000000,0.000000,0.000000" "0.000000,90.000000,0.000000" _alpha) false false)))
    (else
      (Development|PrintString "Locked"))))

(event Custom|DoorOfficeOpened
  (bind _output_get (Variables|Default|SetDoorsOpenedCount (Variables|Default|GetDoorsOpenedCount)))
  (if (== (+ _output_get 2) 4)
    (if (== (+ (Variables|Default|GetDoorsOpenedCount) 0 1 1) 2)
      (Class|BPIInteractable|Interact(Message) (Variables|Default|GetMainDoorRef)))))

(event EventBeginPlay)

(event Collision|EventActorBeginOverlap
  (params (OtherActor :type Actor%20Object%20Reference)))

(event EventTick
  (params (DeltaSeconds :type Float%20%28single-precision%29)))

(fn ConstructionScript)